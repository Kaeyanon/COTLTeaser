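; BP_ToonLight feeds the direction of a referenced Sunlight actor to the toon shading material parameter collection.
; It writes the negated forward vector of Sunlight to the LightDirection parameter in MPC_Toon, skipping the write when the reference is invalid.
; UpdateLighting runs on BeginPlay and every Tick, while the construction script repeats the same logic so the value also updates when the actor is constructed.
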(event `self.ReceiveBeginPlay`
  (`self.UpdateLighting` :!label _label))

(event `self.ReceiveTick`
  (params (DeltaSeconds :type "Float (single-precision)"))
  (goto _label))

(fn `UpdateLighting`
  (if (`KismetSystemLibrary.IsValid` (`self.Sunlight`))
    (`KismetMaterialLibrary.SetVectorParameterValue` "/Game/Blueprint/OutlineShader/MPC_Toon.MPC_Toon" "LightDirection" (`KismetMathLibrary.Conv_VectorToLinearColor` (* (`self.GetActorForwardVector` (`self.Sunlight`)) (-1.0 -1.0 -1.0))))))

(fn `UserConstructionScript`
  (if (`KismetSystemLibrary.IsValid` (`self.Sunlight`))
    (`KismetMaterialLibrary.SetVectorParameterValue` "/Game/Blueprint/OutlineShader/MPC_Toon.MPC_Toon" "LightDirection" (`KismetMathLibrary.Conv_VectorToLinearColor` (* (`self.GetActorForwardVector` (`self.Sunlight`)) (-1.0 -1.0 -1.0))))))